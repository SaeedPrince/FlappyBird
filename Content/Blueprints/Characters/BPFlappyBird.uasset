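; BPFlappyBird is a Flappy Bird character Blueprint with a jump override and debug helpers.
; CanJumpInternal always returns true, so the standard grounded and jump-count checks do not block mid-air flaps.
; CalcSpeed prints the change in X location since its previous call, a per-call delta not divided by time, then stores the current X.
; A PrintonScreen event forwards its arguments to PrintString for screen or log output.
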(event EventPrintonScreen
  (params (inString :type String) (bScreen :type Boolean) (bLog :type Boolean) (inColor :type Linear%20Color%20Structure%20%28by%20ref%29) (inDuration :type Float%20%28single-precision%29))
  (Development|PrintString inString bScreen bLog inColor inDuration))

(fn ConstructionScript)

(fn CanJumpInternal
  (return true))

(fn CalcSpeed
  (bind _returnvalue (Transformation|GetActorLocation))
  (bind _x (Math|Vector|BreakVector _returnvalue))
  (Development|PrintString (Utilities|String|ToString(Float) (- _x (Variables|Default|GetPrevLoc))))
  (Variables|Default|SetPrevLoc _x))